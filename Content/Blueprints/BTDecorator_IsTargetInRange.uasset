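; Behavior tree decorator that checks whether a monster's target is within range.
; It passes only while the controlled BP_Monster has health above zero and its distance to the blackboard Target actor is at most the Range variable.
; A dead monster fails the check.
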(fn `PerformConditionCheckAI`
  (params (OwnerController :type "AIController Object Reference") (ControlledPawn :type "Pawn Object Reference"))
  (returns (ReturnValue :type Boolean))
  (bind _asbp_monster (cast `/Game/Blueprints/BP_Monster` ControlledPawn))
  (if (> (`/Game/Blueprints/BP_Monster.CurHp` _asbp_monster) 0.0)
    (return (<= (`KismetMathLibrary.VSize` (- (`Actor.K2_GetActorLocation` ControlledPawn) (`Actor.K2_GetActorLocation` (`BTFunctionLibrary.GetBlackboardValueAsActor` (`self.Target`))))) (`self.Range`)))
    (else
      (return false))))